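; BP_tenacle is an interactable level actor that the player can remove by pressing Interact while near it.
; Its Box overlap with Player_RebelX enables input and shows an "[E] Interact" crosshair prompt through the HUD, and end overlap by a Character reverses both.
; Interact destroys the actor if the player's Numchemical is zero or more, without decrementing that count.
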(event `self.Box.OnComponentBeginOverlap`
  (params (OverlappedComponent :type "PrimitiveComponent Object Reference") (OtherActor :type "Actor Object Reference") (OtherComp :type "PrimitiveComponent Object Reference") (OtherBodyIndex :type Integer) (bFromSweep :type Boolean) (SweepResult :type "HitResult Structure (by ref)"))
  (bind _asplayer_rebel_x (cast `/Game/RebelX_Core/Blueprints/Player_RebelX` OtherActor))
  (`self.EnableInput` (`GameplayStatics.GetPlayerController` 0))
  (message `/Game/RebelX_Core/Blueprints/Interfaces/BPI_HUD.ShowCrosshairPrompt` (`/Game/RebelX_Core/Blueprints/Player_RebelX.GetAttachedHUD` _asplayer_rebel_x) "[E] Interact" "NewEnumerator0" 0.0 false (struct)))

(event `InputAction|Interact`
  (params (Key :type "Key Structure"))
  (:`Pressed`
    (bind _asplayer_rebel_x (cast `/Game/RebelX_Core/Blueprints/Player_RebelX` (stale `self.Box.OnComponentBeginOverlap` OtherActor)))
    (if (>= (`/Game/RebelX_Core/Blueprints/Player_RebelX.Numchemical` _asplayer_rebel_x) 0.0)
      (`self.K2_DestroyActor`))))

(event `self.Box.OnComponentEndOverlap`
  (params (OverlappedComponent :type "PrimitiveComponent Object Reference") (OtherActor :type "Actor Object Reference") (OtherComp :type "PrimitiveComponent Object Reference") (OtherBodyIndex :type Integer))
  (cast `Character` OtherActor)
  (`self.DisableInput` (`GameplayStatics.GetPlayerController` 0))
  (message `/Game/RebelX_Core/Blueprints/Interfaces/BPI_HUD.HideCrosshairPrompt` (`/Game/RebelX_Core/Blueprints/Player_RebelX.GetAttachedHUD` (stale `self.Box.OnComponentBeginOverlap` _asplayer_rebel_x))))

(fn `UserConstructionScript`)