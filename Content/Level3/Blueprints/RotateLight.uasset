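; RotateLight is a rotating light actor for Level3, with a sphere bulb and two spotlights.
; On BeginPlay, a fast looping timer, used in place of Tick, pitches the sphere by a step scaled by RotateSpeed, without delta-time compensation.
; A SetGreen event recolors both spotlights and swaps the sphere's material to a green variant.
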(event `self.ReceiveBeginPlay`
  (`KismetSystemLibrary.K2_SetTimerDelegate` (delegate `RotateBulb`) 0.01 true))

(event `RotateBulb`
  (`SceneComponent.K2_AddLocalRotation` (`self.Sphere`) (`KismetMathLibrary.MakeRotator` 0.0 (* 1.5 (`self.RotateSpeed`))) false false))

(event `SetGreen`
  (`LightComponent.SetLightColor` (`self.SpotLight`) (`self.greenLightColor`) true)
  (`LightComponent.SetLightColor` (`self.SpotLight1`) (`self.greenLightColor`) true)
  (`PrimitiveComponent.SetMaterial` (`self.Sphere`) 0 "/Game/Level3/Materials/YifanCreated/GreenLight.GreenLight"))

(fn `UserConstructionScript`)