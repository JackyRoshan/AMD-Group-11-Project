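; BP_tenacle_2 is a tentacle obstacle in Level 3 that the player clears with Interact once its connected eggs are gone.
; Box overlap enables input and shows a HUD prompt based on EggCount, which starts at the egg array length and is not decremented here.
; Clearing checks Numchemical >= 0 without consuming it, plays sound and shake, damages any connected boss, then destroys the tentacle.
; A separate wakeUpEggs event enables spawning on the eggs.
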(event `self.ReceiveBeginPlay`
  (set `self.EggCount` (`KismetArrayLibrary.Array_Length` (`self.connectedEggs`))))

(event `self.Box.OnComponentBeginOverlap`
  (params (OverlappedComponent :type "PrimitiveComponent Object Reference") (OtherActor :type "Actor Object Reference") (OtherComp :type "PrimitiveComponent Object Reference") (OtherBodyIndex :type Integer) (bFromSweep :type Boolean) (SweepResult :type "HitResult Structure (by ref)"))
  (bind _asplayer_rebel_x (cast `/Game/RebelX_Core/Blueprints/Player_RebelX` OtherActor))
  (`self.EnableInput` (`GameplayStatics.GetPlayerController` 0))
  (if (<= (`self.EggCount`) 0)
    (bind _ashud_rebel_x (`/Game/RebelX_Core/Blueprints/Player_RebelX.GetAttachedHUD` _asplayer_rebel_x))
    (message `/Game/RebelX_Core/Blueprints/Interfaces/BPI_HUD.ShowCrosshairPrompt` _ashud_rebel_x "[E] Clear tentacle using item" "NewEnumerator0" 0.0 false (struct))
    (else
      (message `/Game/RebelX_Core/Blueprints/Interfaces/BPI_HUD.ShowCrosshairPrompt` _ashud_rebel_x "Eggs not cleared yet" "NewEnumerator1" 0.0 false (struct)))))

(event `wakeUpEggs`
  (for _array_element (`self.connectedEggs`)
    (set `/Game/Enemy/MonsterEgg.canSpawn` true _array_element)))

(event `self.Box.OnComponentEndOverlap`
  (params (OverlappedComponent :type "PrimitiveComponent Object Reference") (OtherActor :type "Actor Object Reference") (OtherComp :type "PrimitiveComponent Object Reference") (OtherBodyIndex :type Integer))
  (cast `Character` OtherActor)
  (`self.DisableInput` (`GameplayStatics.GetPlayerController` 0))
  (message `/Game/RebelX_Core/Blueprints/Interfaces/BPI_HUD.HideCrosshairPrompt` (`/Game/RebelX_Core/Blueprints/Player_RebelX.GetAttachedHUD` (stale `self.Box.OnComponentBeginOverlap` _asplayer_rebel_x))))

(event `InputAction|Interact`
  (params (Key :type "Key Structure"))
  (:`Pressed`
    (if (<= (`self.EggCount`) 0)
      (bind _asplayer_rebel_x (cast `/Game/RebelX_Core/Blueprints/Player_RebelX` (`GameplayStatics.GetPlayerCharacter` 0)))
      (if (>= (`/Game/RebelX_Core/Blueprints/Player_RebelX.Numchemical` _asplayer_rebel_x) 0.0)
        (`self.DisableTentacle`)))))

(event `DisableTentacle`
  (bind _returnvalue (`self.K2_GetActorLocation`))
  (bind _connectedboss (`self.connectedBoss`))
  (`|ExecutionSequence`
    (:`then_0`
      (if (`self.IsFirstTentacle`)
        (message `/Game/RebelX_Core/Blueprints/Interfaces/BPI_HUD.UpdateObjective` (`PlayerController.GetHUD` (`GameplayStatics.GetPlayerController` 0)) "#$%!@#$!@$#%" "What is ahead...!?"))
      (`GameplayStatics.PlaySoundAtLocation` "/Game/Level3/Audio/Huge_Monster_Death_01.Huge_Monster_Death_01" _returnvalue (struct) 1.0 1.0 0.0 null null null null)
      (`GameplayStatics.PlayWorldCameraShake` "/Game/Level3/Blueprints/BP_NewCameraShake.BP_NewCameraShake_C" _returnvalue 0.0 5000.0)
      (`/Engine/EditorBlueprintResources/StandardMacros.IsValid` _connectedboss
        (:`Is Valid`
          (set `/Game/Level3/Blueprints/BP_Boss.currentHealth` (- (`/Game/Level3/Blueprints/BP_Boss.currentHealth` _connectedboss) 2000.0) _connectedboss))
        (:`Is Not Valid`
          _))
      (`self.K2_DestroyActor`))))

(fn `UserConstructionScript`)