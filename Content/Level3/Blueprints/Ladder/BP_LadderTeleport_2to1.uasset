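; Level 3 ladder teleport actor that moves the player downstairs, from 2 to 1 per its name.
; Overlapping StartPos with Player_RebelX enables the actor's input and shows an "[E] Go Downstair" crosshair prompt on the HUD.
; Pressing Interact sets player character 0's location to EndPos, with no sweep.
; Leaving StartPos disables input and hides the prompt.
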(event `self.StartPos.OnComponentBeginOverlap`
  (params (OverlappedComponent :type "PrimitiveComponent Object Reference") (OtherActor :type "Actor Object Reference") (OtherComp :type "PrimitiveComponent Object Reference") (OtherBodyIndex :type Integer) (bFromSweep :type Boolean) (SweepResult :type "HitResult Structure (by ref)"))
  (bind _asplayer_rebel_x (cast `/Game/RebelX_Core/Blueprints/Player_RebelX` OtherActor))
  (`self.EnableInput` (`GameplayStatics.GetPlayerController` 0))
  (message `/Game/RebelX_Core/Blueprints/Interfaces/BPI_HUD.ShowCrosshairPrompt` (`/Game/RebelX_Core/Blueprints/Player_RebelX.GetAttachedHUD` _asplayer_rebel_x) "[E] Go Downstair" "NewEnumerator0" 0.0 false (struct)))

(event `InputAction|Interact`
  (params (Key :type "Key Structure"))
  (:`Pressed`
    (`self.K2_SetActorLocation` (`GameplayStatics.GetPlayerCharacter` 0) (`SceneComponent.K2_GetComponentLocation` (`self.EndPos`)) false false)))

(event `self.StartPos.OnComponentEndOverlap`
  (params (OverlappedComponent :type "PrimitiveComponent Object Reference") (OtherActor :type "Actor Object Reference") (OtherComp :type "PrimitiveComponent Object Reference") (OtherBodyIndex :type Integer))
  (cast `/Game/RebelX_Core/Blueprints/Player_RebelX` OtherActor)
  (`self.DisableInput` (`GameplayStatics.GetPlayerController` 0))
  (message `/Game/RebelX_Core/Blueprints/Interfaces/BPI_HUD.HideCrosshairPrompt` (`/Game/RebelX_Core/Blueprints/Player_RebelX.GetAttachedHUD` (stale `self.StartPos.OnComponentBeginOverlap` _asplayer_rebel_x))))

(fn `UserConstructionScript`)