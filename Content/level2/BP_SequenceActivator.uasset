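; Level 2 trigger actor that starts a level sequence and cabin dialogue when the Player_RebelX character enters its box.
; A DoOnce-gated overlap plays the sequence and a loud coughing sound, then calls TalkCabin2 after a short delay.
; TalkCabin2 advances a counter into parallel text and sound arrays, showing each line in a Dialoglevel2 widget with its voice clip.
; The End flag removes the widget after a delay.
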(event `self.Box.OnComponentBeginOverlap`
  (params (OverlappedComponent :type "PrimitiveComponent Object Reference") (OtherActor :type "Actor Object Reference") (OtherComp :type "PrimitiveComponent Object Reference") (OtherBodyIndex :type Integer) (bFromSweep :type Boolean) (SweepResult :type "HitResult Structure (by ref)"))
  (cast `/Game/RebelX_Core/Blueprints/Player_RebelX` OtherActor)
  (`/Engine/EditorBlueprintResources/StandardMacros.DoOnce` false
    (:`Completed`
      (bind _outactor (`LevelSequencePlayer.CreateLevelSequencePlayer` (`self.Level Sequence`)))
      (`MovieSceneSequencePlayer.Play` (`LevelSequenceActor.SequencePlayer` _outactor))
      (`GameplayStatics.PlaySound2D` "/Game/level2/Dialog/Coughing.Coughing" 5.0 1.0 0.0 null null)
      (`KismetSystemLibrary.Delay` 1.0)
      (`self.TalkCabin2` true))))

(event `TalkCabin2`
  (params (`End?` :type Boolean))
  (set `self.End?` `End?`)
  (`/Engine/EditorBlueprintResources/StandardMacros.IncrementInt` (`self.TalkCountCabin2`)
    (:`  `
      (if (<= (`self.TalkCountCabin2`) (`KismetArrayLibrary.Array_Length` (`self.DialogCabin2`)))
        (`self.UI`
          (:`then`
            _)
          (:`else`
            (bind _returnvalue (`|CreateWidget` "/Game/level2/Dialog/Dialoglevel2.Dialoglevel2_C" (`GameplayStatics.GetPlayerController` 0)))
            (bind _output_get (set `self.UI` _returnvalue))
            (`UserWidget.AddToViewport` _output_get 0)))
        (`TextBlock.SetText` (`/Game/level2/Dialog/Dialoglevel2.TalkText` (`self.UI`)) (`KismetTextLibrary.Conv_StringToText` (`|GetArrayItem` (`self.DialogCabin2`) (`self.TalkCountCabin2`))))
        (`|ExecutionSequence`
          (:`then_0`
            (if (`self.End?`)
              (`KismetSystemLibrary.Delay` 6.0)
              (`Widget.RemoveFromParent` (`self.UI`))))
          (:`then_1`
            (`GameplayStatics.PlaySound2D` (`|GetArrayItem` (`self.DialogSoundCabin2`) (`self.TalkCountCabin2`)) 1.0 1.0 0.0 null null)))
        (else
          (`Widget.RemoveFromParent` (`self.UI`)))))))

(fn `UserConstructionScript`)